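; Arrow burst emitter actor that continuously fires BP_Arrow projectiles from its Arrow component's location and rotation.
; A fast looping timer started on BeginPlay drives the spawning, ignoring collision at the spawn point.
; It also registers itself as the CollisionHandler object on BP_MonsterSpawn's NSMonsterOnce Niagara system.
; The exported particle data it receives back only prints a debug "Hit" per entry.
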(event Custom|Spawn
  (bind _arrow (Variables|Default|GetArrow))
  (Game|SpawnActorfromClass "/Game/xuli/BP_Arrow.BP_Arrow_C" (Math|Transform|MakeTransform (Transformation|GetWorldLocation _arrow) (Transformation|GetWorldRotation _arrow) "1.000000,1.000000,1.000000") "AlwaysSpawn" "MultiplyWithRoot" 0 0))

(event EventBeginPlay
  (Utilities|Time|SetTimerbyEvent (delegate Custom|Spawn) 0.1 true)
  (bind _returnvalue (Actor|GetActorOfClass "/Game/xuli/BP_MonsterSpawn.BP_MonsterSpawn_C"))
  (Class|NiagaraComponent|SetVariableObject (Variables|/Game/xuli/BP_MonsterSpawn.BP_MonsterSpawn_C|GetNS_MonsterOnce _returnvalue) "CollisionHandler" self))

(event Collision|EventActorBeginOverlap
  (params (OtherActor :type Actor%20Object%20Reference)))

(event EventTick
  (params (DeltaSeconds :type Float%20%28single-precision%29)))

(event EventParticleData
  (params (Data :type Array%20of%20Basic%20Particle%20Data%20Structures) (NiagaraSystem :type Niagara%20System%20Object%20Reference) (SimulationPositionOffset :type Vector%20%28by%20ref%29 :default "0, 0, 0"))
  (for _array_element Data
    (Development|PrintString "Hit" true true "(R=0.000000,G=0.660000,B=1.000000,A=1.000000)" 0.5)))

(fn ConstructionScript)