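; BP_MonsterSpawn is an actor that drives a Niagara-based monster effect and counts particle deaths.
; On BeginPlay it finds the BP_ArrowBrust actor, registers itself as the system's DeathHandler and shows the UMG_KillNum widget.
; Each tick it feeds that actor's location to Niagara as Target.
; Exported particle data returns through the ParticleData callback, where each entry with non-positive Size prints "Death" and increments the counter Int.
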(event EventBeginPlay
  (bind _returnvalue (Actor|GetActorOfClass "/Game/xuli/BP_ArrowBrust.BP_ArrowBrust_C"))
  (Variables|Default|SetTarget _returnvalue)
  (Class|NiagaraComponent|SetVariableObject (Variables|Default|GetNS_MonsterOnce) "DeathHandler" self)
  (bind _returnvalue_2 (UserInterface|CreateWidget "/Game/xuli/UMG_KillNum.UMG_KillNum_C"))
  (UserInterface|Viewport|AddtoViewport _returnvalue_2 0))

(event Collision|EventActorBeginOverlap
  (params (OtherActor :type Actor%20Object%20Reference)))

(event EventTick
  (params (DeltaSeconds :type Float%20%28single-precision%29))
  (Class|NiagaraComponent|SetVariablePosition (Variables|Default|GetNS_MonsterOnce) "Target" (Transformation|GetActorLocation (Variables|Default|GetTarget))))

(event EventParticleData
  (params (Data :type Array%20of%20Basic%20Particle%20Data%20Structures) (NiagaraSystem :type Niagara%20System%20Object%20Reference) (SimulationPositionOffset :type Vector%20%28by%20ref%29 :default "0, 0, 0"))
  (for _array_element Data
    (if (<= (.Size (Utilities|Struct|BreakBasicParticleData _array_element)) 0.0)
      (Development|PrintString "Death" true true "(R=1.000000,G=0.048928,B=0.000000,A=1.000000)" 2.0 "Death")
      (Math|Integer|IncrementInt (Variables|Default|GetInt)))))

(fn ConstructionScript)